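; BP_SlingshotRock is the rock actor for an enemy slingshot ability, tumbling visually while it exists.
; BeginPlay picks random yaw, pitch and roll rates, which Tick scales by delta time to spin RockMesh in local space.
; A short delay after spawn switches SphereComponent collision to query-only.
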(event EventBeginPlay
  (bind _returnvalue (Math|Random|RandomFloatinRange -5e+02 5e+02))
  (Variables|Default|SetYawRotationRate _returnvalue)
  (Variables|Default|SetPitchRotationRate _returnvalue)
  (Variables|Default|SetRollRotationRate _returnvalue)
  (Utilities|FlowControl|Delay 0.1)
  (Collision|SetCollisionEnabled (Variables|Default|GetSphereComponent) "QueryOnly"))

(event EventTick
  (params (DeltaSeconds :type Float%20%28single-precision%29))
  (Transformation|AddLocalRotation (Variables|Default|GetRockMesh) (Math|Rotator|MakeRotator (* (Variables|Default|GetRollRotationRate) DeltaSeconds) (* (Variables|Default|GetPitchRotationRate) DeltaSeconds) (* (Variables|Default|GetYawRotationRate) DeltaSeconds)) false false))

(fn ConstructionScript)